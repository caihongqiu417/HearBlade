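; Preview actor for the Dragon Knight enemy that shows its first combo attack animation, Combo01, on a fully dressed modular character.
; The construction script attaches the sword and Niagara fire effects to body sockets and makes the body, gauntlets, greaves and head follow the cape body mesh's pose.
; On BeginPlay, skeletal meshes tagged ComboPreview play the combo montage once without looping.
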(event EventBeginPlay
  (for _array_element (Actor|GetComponentsbyTag "/Script/Engine.SkeletalMeshComponent" "ComboPreview")
    (bind _as骨骼网格体组件 (Utilities|Casting|CastToSkeletalMeshComponent _array_element))
    (Components|Animation|PlayAnimation _as骨骼网格体组件 "/Game/Enemies/DF_DRAGON_KNIGHT/Montage/Combo01_Montage.Combo01_Montage" false)))

(event Collision|EventActorBeginOverlap
  (params (OtherActor :type Actor%20Object%20Reference)))

(event EventTick
  (params (DeltaSeconds :type Float%20%28single-precision%29)))

(fn ConstructionScript
  (bind _ue5_body_cape (Variables|Default|GetUE5_body_cape))
  (Transformation|AttachComponentToComponent (Variables|Default|GetUE5_sword) _ue5_body_cape "hand_r" "KeepRelative" "KeepRelative" "SnapToTarget" true)
  (Transformation|AttachComponentToComponent (Variables|Default|GetNS_arms_Fire_l) _ue5_body_cape "upperarm_l" "KeepRelative" "KeepRelative" "SnapToTarget" true)
  (Transformation|AttachComponentToComponent (Variables|Default|GetNS_shoulder_Fire_r) _ue5_body_cape "upperarm_r" "KeepRelative" "KeepRelative" "KeepRelative" true)
  (Transformation|AttachComponentToComponent (Variables|Default|GetNS_chest_Fire) _ue5_body_cape "spine_04" "KeepRelative" "KeepRelative" "KeepRelative" true)
  (Transformation|AttachComponentToComponent (Variables|Default|GetNS_head_Fire) _ue5_body_cape "head" "KeepRelative" "KeepRelative" "KeepRelative" true)
  (Components|SkinnedMesh|SetLeaderPoseComponent (Variables|Default|GetUE5_body) (Variables|Default|GetUE5_body_cape) false false))